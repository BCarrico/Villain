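; GA_TestProjectileAbility_LeftHanded is a test gameplay ability that fires a projectile toward the target under the mouse.
; It commits, stores the cursor hit location, then plays the FireBolt section of the fire-weapon montage.
; A wait for the Event.Montage.Test gameplay event times the projectile spawn from the weapon combat socket, with a debug print.
; Montage completion ends the ability.
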(event `self.K2_ActivateAbility`
  (`self.K2_CommitAbility`)
  (bind (_asynctaskproxy _datahandle) (`TargetDataUnderMouse.CreateTargetDataUnderMouse`)
    (:`ValidData`
      (set `self.ProjectileTargetLocation` (`.Location` (`GameplayStatics.BreakHitResult` (`AbilitySystemBlueprintLibrary.GetHitResultFromTargetData` _datahandle))))
      (`AbilityTask_PlayMontageAndWait.CreatePlayMontageAndWaitProxy` "None" "/Game/Assets/Animations/AM_FireWeapon.AM_FireWeapon" 1.0 "FireBolt" false
        (:`then`
          (`AbilityTask_WaitGameplayEvent.WaitGameplayEvent` (struct :`TagName` "Event.Montage.Test") null
            (:`EventReceived`
              (`self.SpawnProjectile` (`self.ProjectileTargetLocation`) (`BlueprintGameplayTagLibrary.MakeLiteralGameplayTag` (struct :`TagName` "CombatSocket.Weapon")))
              (`KismetSystemLibrary.PrintString` "Activate Ability (BP)"))))
        (:`OnCompleted`
          (`self.K2_EndAbility`))))))