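; Gameplay ability that fires a projectile at the point under the mouse and kicks the villain character backward with recoil.
; It saves the target, turns player 0's control yaw toward it and plays the fire montage from its RifleAim section.
; A montage gameplay event spawns the projectile from the weapon socket and applies a velocity-change impulse opposite facing, scaled by RecoilStrength.
; The ability ends only when the montage completes.
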(event `self.K2_ActivateAbility`
  (bind _returnvalue (`self.GetAvatarActorFromActorInfo`))
  (bind _villaincharacter (`self.VillainCharacter`))
  (bind (_returnvalue_roll _returnvalue_pitch _returnvalue_yaw) (`KismetMathLibrary.BreakRotator` (`KismetMathLibrary.FindLookAtRotation` (`Actor.K2_GetActorLocation` _returnvalue) (`self.ProjectileTargetLocation`))))
  (`self.K2_CommitAbility`)
  (bind (_asynctaskproxy _datahandle) (`TargetDataUnderMouse.CreateTargetDataUnderMouse`)
    (:`then`
      (set `self.ProjectileTargetLocation` (`.Location` (`GameplayStatics.BreakHitResult` (`AbilitySystemBlueprintLibrary.GetHitResultFromTargetData` _datahandle))))
      (bind _asvillain_character (cast `VillainCharacter` _returnvalue))
      (set `self.VillainCharacter` _asvillain_character)
      (`Controller.SetControlRotation` (`GameplayStatics.GetPlayerController` 0) (`KismetMathLibrary.MakeRotator` 0.0 0.0 _returnvalue_yaw))
      (set `Pawn.bUseControllerRotationYaw` true (`self.VillainCharacter`))
      (`AbilityTask_PlayMontageAndWait.CreatePlayMontageAndWaitProxy` "None" "/Game/Assets/Animations/AM_FireWeapon.AM_FireWeapon" 1.0 "RifleAim" false
        (:`then`
          (`AbilityTask_WaitGameplayEvent.WaitGameplayEvent` (struct :`TagName` "Event.Montage.Test") null true
            (:`EventReceived`
              (`self.SpawnProjectile` (`self.ProjectileTargetLocation`) (`BlueprintGameplayTagLibrary.MakeLiteralGameplayTag` (struct :`TagName` "CombatSocket.Weapon")))
              (bind _returnvalue_2 (`self.GetOppositeFacingDirection` _villaincharacter))
              (`CharacterMovementComponent.AddImpulse` (`Character.CharacterMovement` _villaincharacter) _returnvalue_2 true)
              (`KismetSystemLibrary.PrintString` "Hello"))))
        (:`OnCompleted`
          (`self.K2_EndAbility`))))))

(fn `GetOppositeFacingDirection`
  (params (Actor :type "Character Object Reference"))
  (returns (ReturnValue :type "Vector Structure"))
  (return (* (`KismetMathLibrary.NegateVector` (`Actor.GetActorForwardVector` Actor)) (`self.RecoilStrength`))))