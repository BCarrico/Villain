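; Rifle gameplay ability that fires a projectile at the point under the mouse cursor.
; On valid target data it yaws the controller toward the hit location, enables controller-yaw rotation on the VillainCharacter and plays the fire montage.
; A montage gameplay event times the projectile spawn from the weapon socket.
; The ability ends when the montage completes or is interrupted, switching controller-yaw rotation back off.
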(event `self.K2_ActivateAbility`
  (`self.StoreKeyVariables`)
  (`self.K2_CommitAbility`)
  (bind (_asynctaskproxy _datahandle) (`TargetDataUnderMouse.CreateTargetDataUnderMouse`)
    (:`ValidData`
      (set `self.ProjectileTargetLocation` (`.Location` (`GameplayStatics.BreakHitResult` (`AbilitySystemBlueprintLibrary.GetHitResultFromTargetData` _datahandle))))
      (`self.RotatePlayerTowardsTarget`)
      (`AbilityTask_PlayMontageAndWait.CreatePlayMontageAndWaitProxy` "None" "/Game/Assets/Animations/AM_FireWeapon.AM_FireWeapon" 1.0 "RifleAim" false
        (:`then`
          (`AbilityTask_WaitGameplayEvent.WaitGameplayEvent` (struct :`TagName` "Event.Montage.Test") null true
            (:`EventReceived`
              (`self.SpawnProjectile` (`self.ProjectileTargetLocation`) (`BlueprintGameplayTagLibrary.MakeLiteralGameplayTag` (struct :`TagName` "CombatSocket.Weapon"))))))
        (:`OnCompleted`
          (`self.K2_EndAbility` :!label _label))
        (:`OnInterrupted`
          (goto _label))))))

(event `self.K2_OnEndAbility`
  (params (bWasCancelled :type Boolean))
  (set `Pawn.bUseControllerRotationYaw` false (`self.As Villain Character`)))

(fn `RotatePlayerTowardsTarget`
  (bind (_returnvalue_roll _returnvalue_pitch _returnvalue_yaw) (`KismetMathLibrary.BreakRotator` (`KismetMathLibrary.FindLookAtRotation` (`Actor.K2_GetActorLocation` (`self.GetAvatarActorFromActorInfo`)) (`self.ProjectileTargetLocation`))))
  (`Controller.SetControlRotation` (`GameplayStatics.GetPlayerController` 0) (`KismetMathLibrary.MakeRotator` 0.0 0.0 _returnvalue_yaw))
  (set `Pawn.bUseControllerRotationYaw` true (`self.As Villain Character`)))

(fn `StoreKeyVariables`
  (bind _asvillain_character (cast `VillainCharacter` (`self.GetAvatarActorFromActorInfo`)))
  (set `self.As Villain Character` _asvillain_character)
  (set `self.CombatComponent` (`VillainCharacter.Combat` _asvillain_character)))