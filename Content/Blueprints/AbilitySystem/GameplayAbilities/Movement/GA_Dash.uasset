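; Gameplay ability that makes the villain character perform a quick dash.
; It commits, applies an input-blocking effect, then dashes along pending input if moving horizontally, or along actor forward if not.
; Both branches play the flying dash montage alongside a short constant root motion force that maintains its last velocity on finish.
; The ability ends when either the force or montage finishes, and stops the montage on end.
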(event `self.K2_ActivateAbility`
  (bind _returnvalue (`self.GetAvatarActorFromActorInfo`))
  (`self.K2_CommitAbility`)
  ;[1 1 1] Duration Based on Apply Root Motion Constant DURATION Length
  (`self.BP_ApplyGameplayEffectToOwner` "/Game/Blueprints/AbilitySystem/GameplayEffects/GE_BlockInput.GE_BlockInput_C")
  (bind _asvillain_character (cast `VillainCharacter` (`self.GetAvatarActorFromActorInfo`)))
  (bind _charactermovement (`Character.CharacterMovement` _asvillain_character))
  ;[1 1 1] Is character moving? Dash that direction, if not, dash where facing
  (if (> (`KismetMathLibrary.VSizeXY` (`MovementComponent.Velocity` _charactermovement)) 0.0)
    (`AbilityTask_PlayMontageAndWait.CreatePlayMontageAndWaitProxy` "None" "/Game/Assets/Animations/AM_FlyingDash.AM_FlyingDash" 1.0 "None" false
      (:`then`
        (`AbilityTask_ApplyRootMotionConstantForce.ApplyRootMotionConstantForce` "None" (`PawnMovementComponent.GetPendingInputVector` _charactermovement) 3500.0 0.1 false null "MaintainLastRootMotionVelocity" (`Actor.GetVelocity` (`self.GetAvatarActorFromActorInfo`))
          (:`OnFinish`
            (`self.K2_EndAbility` :!label _label))))
      (:`OnCompleted`
        (`self.K2_EndAbility` :!label _label_2))
      (:`OnBlendOut`
        (goto _label_2))
      (:`OnInterrupted`
        (goto _label_2))
      (:`OnCancelled`
        (goto _label_2)))
    (else
      (`AbilityTask_PlayMontageAndWait.CreatePlayMontageAndWaitProxy` "None" "/Game/Assets/Animations/AM_FlyingDash.AM_FlyingDash" 1.0 "None" false
        (:`then`
          (`AbilityTask_ApplyRootMotionConstantForce.ApplyRootMotionConstantForce` "None" (`Actor.GetActorForwardVector` _returnvalue) 3500.0 0.1 false null "MaintainLastRootMotionVelocity" (`Actor.GetVelocity` _returnvalue)
            (:`OnFinish`
              (goto _label))))
        (:`OnCompleted`
          _)
        (:`OnBlendOut`
          _)
        (:`OnInterrupted`
          _)
        (:`OnCancelled`
          _))
      (`self.K2_EndAbility`))))

(event `self.K2_OnEndAbility`
  (params (bWasCancelled :type Boolean))
  (`self.MontageStop` -1.0))